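; BP_BaseWeapon is a base weapon actor that fires bullets for the pawn it is attached to as a child actor.
; On BeginPlay it caches its parent actor as the owning pawn, printing a debug message if that cast fails.
; Attack spawns the Bullet class at the muzzle socket, using the pawn's base aim rotation and setting it as instigator.
; PawnDied only sets a dead flag, which Attack does not check.
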(event Custom|Attack
  (Game|SpawnActorfromClass (Variables|Default|GetBullet) (Math|Transform|MakeTransform (Transformation|GetSocketLocation (Variables|Default|GetSkeletalMesh) "MuzzleFlashSocket") (Pawn|GetBaseAimRotation (Variables|Default|GetPawnOwner)) "1,1,1") "Undefined" 0 (Variables|Default|GetPawnOwner)))

(event Custom|PawnDied
  (Variables|Default|SetPawnDead true))

(event EventBeginPlay
  (bind _aspawn (Utilities|Casting|CastToPawn (Actor|GetParentActor))
    (:then
      (Variables|Default|SetPawnOwner _aspawn))
    (:CastFailed
      (Development|PrintString "No Bullet"))))

(fn ConstructionScript)