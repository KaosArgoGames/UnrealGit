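; BP_BaseBullet is a base bullet actor that applies damage to whatever its BulletCollider overlaps.
; The construction script sets the collider's world scale from Size, and BeginPlay starts a one-shot timer of TimeToDestroy length, with no handler body shown.
; On overlap it passes Damage with the instigator's controller and the instigator as damage causer, prints both names, then destroys itself.
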(event OnComponentBeginOverlap(BulletCollider)
  (params (OverlappedComponent :type Primitive%20Component%20Object%20Reference) (OtherActor :type Actor%20Object%20Reference) (OtherComp :type Primitive%20Component%20Object%20Reference) (OtherBodyIndex :type Integer) (bFromSweep :type Boolean) (SweepResult :type Hit%20Result%20Structure%20%28by%20ref%29))
  (bind _returnvalue (Game|GetInstigator))
  (bind _returnvalue_2 (Game|GetInstigatorController))
  (Game|Damage|ApplyDamage OtherActor (Variables|Default|GetDamage) _returnvalue_2 _returnvalue)
  (Development|PrintString (Utilities|String|Append (Utilities|GetDisplayName _returnvalue_2) (Utilities|GetDisplayName _returnvalue)))
  (Actor|DestroyActor))

(event EventBeginPlay
  (Utilities|Time|SetTimerbyEvent (EventDispatchers|CreateEvent :!event K2DestroyActor) (Variables|Default|GetTimeToDestroy)))

(fn ConstructionScript
  (Transformation|SetWorldScale3D (Variables|Default|GetBulletCollider) (LocalVariables|GetSize)))