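; BP_Player is the player actor that carries a weapon and forwards attacks to it.
; On BeginPlay it spawns WeaponClass through a child actor component and caches it as a BP_BaseWeapon, then caches the mesh's ABP_Rifle anim instance, printing a message if either cast fails.
; Attack calls the weapon's Attack, then PersonaUpdate on the anim blueprint.
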(event Custom|Attack
  (Default|Attack (Variables|Default|GetWeapon))
  (Class|RifleAnim|PersonaUpdate (Variables|Default|GetAnim%20BP)))

(event EventBeginPlay
  (bind _weaponchildactor (Variables|Default|GetWeaponChildActor))
  (ChildActorComponent|SetChildActorClass _weaponchildactor (Variables|Default|GetWeaponClass))
  (bind _asbp_base_weapon (Utilities|Casting|CastToBP_BaseWeapon (Variables|/Script/Engine.ChildActorComponent|GetChildActor _weaponchildactor))
    (:then
      (Variables|Default|SetWeapon _asbp_base_weapon)
      (bind _asabp_rifle (Utilities|Casting|CastToABP_Rifle (Components|SkeletalMesh|GetAnimInstance (Variables|Character|GetMesh)))
        (:then
          (Variables|Default|SetAnim%20BP _asabp_rifle))
        (:CastFailed
          (Development|PrintString "Need Animation Set to Rifle"))))
    (:CastFailed
      (Development|PrintString "No Weapon"))))

(fn ConstructionScript)